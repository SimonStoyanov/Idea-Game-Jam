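; Player character Blueprint with movement, mouse look, jumping and laser firing.
; Axis inputs drive movement along the control rotation's yaw, so pitch does not affect it, and feed controller pitch and yaw for looking.
; Left mouse button spawns a Laser actor at the LaserSpawn component's world transform, while the Jump action calls the built-in Jump.
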(event Input|ActionEvents|InputActionJump
  (params (Key :type Key%20Structure))
  ;[1 1 1] Player Jump
  (:Pressed
    (Character|Jump)))

(event Input|AxisEvents|InputAxisMoveForward
  (params (AxisValue :type Float%20%28single-precision%29))
  ;[1 1 1] Player Movement
  (Pawn|Input|AddMovementInput (Math|Vector|GetForwardVector (Math|Rotator|MakeRotator 0.0 0.0 (.Yaw (Math|Rotator|BreakRotator (Pawn|GetControlRotation :!class /Script/Engine.Pawn))))) AxisValue false))

(event Input|AxisEvents|InputAxisMoveRight
  (params (AxisValue :type Float%20%28single-precision%29))
  ;[1 1 1] Player Movement
  (Pawn|Input|AddMovementInput (Math|Vector|GetRightVector (Math|Rotator|MakeRotator 0.0 0.0 (.Yaw (Math|Rotator|BreakRotator (Pawn|GetControlRotation :!class /Script/Engine.Pawn))))) AxisValue false))

(event Input|AxisEvents|InputAxisLookRight
  (params (AxisValue :type Float%20%28single-precision%29))
  ;[1 1 1] Player Rotation
  (Pawn|Input|AddControllerYawInput AxisValue))

(event Input|AxisEvents|InputAxisLookUp
  (params (AxisValue :type Float%20%28single-precision%29))
  ;[1 1 1] Player Rotation
  (Pawn|Input|AddControllerPitchInput AxisValue))

(event Input|MouseEvents|LeftMouseButton
  (params (Key :type Key%20Structure))
  (bind _laserspawn (Variables|Default|GetLaserSpawn))
  ;[1 1 1] Action
  (:Pressed
    (Game|SpawnActorfromClass "/Game/Game/Blueprints/Laser.Laser_C" (Math|Transform|MakeTransform (Transformation|GetWorldLocation _laserspawn) (Transformation|GetWorldRotation _laserspawn)) "Undefined" 0 0)))

(fn ConstructionScript)